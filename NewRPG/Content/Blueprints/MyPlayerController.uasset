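; Player controller that routes melee and movement input to the possessed ThirdPersonCharacter and puts the HUD widget on screen.
; BeginPlay caches the controlled pawn once and creates the HUD, and each input handler casts that cached pawn.
; Non-zero MoveUp and MoveRight axes call their movement functions, then set the character's MoveRotationEnum to one of four directions by sign, while MeleeAttack triggers the character's attack.
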(event `InputAction|MeleeAttack`
  (params (Key :type "Key Structure"))
  (:`Pressed`
    (bind _asthird_person_character (cast `/Game/ThirdPersonBP/Blueprints/ThirdPersonCharacter` (`self.ControlledPawn`)))
    (`/Game/ThirdPersonBP/Blueprints/ThirdPersonCharacter.MeleeAttack` _asthird_person_character)))

(event `InputAxis|MoveRight`
  (params (AxisValue :type "Float (single-precision)"))
  (if (!= AxisValue 0.0)
    (`self.MoveRight` AxisValue)
    (bind _asthird_person_character (cast `/Game/ThirdPersonBP/Blueprints/ThirdPersonCharacter` (`self.ControlledPawn`)))
    (if (> AxisValue 0.0)
      (set `/Game/ThirdPersonBP/Blueprints/ThirdPersonCharacter.MoveRotationEnum` "NewEnumerator2" _asthird_person_character)
      (else
        (set `/Game/ThirdPersonBP/Blueprints/ThirdPersonCharacter.MoveRotationEnum` "NewEnumerator3" _asthird_person_character)))))

(event `InputAxis|MoveUp`
  (params (AxisValue :type "Float (single-precision)"))
  (if (!= AxisValue 0.0)
    (`self.MoveUp` AxisValue)
    (bind _asthird_person_character (cast `/Game/ThirdPersonBP/Blueprints/ThirdPersonCharacter` (`self.ControlledPawn`)))
    (if (> AxisValue 0.0)
      (set `/Game/ThirdPersonBP/Blueprints/ThirdPersonCharacter.MoveRotationEnum` "NewEnumerator0" _asthird_person_character)
      (else
        (set `/Game/ThirdPersonBP/Blueprints/ThirdPersonCharacter.MoveRotationEnum` "NewEnumerator1" _asthird_person_character)))))

(event `self.ReceiveBeginPlay`
  (set `self.ControlledPawn` (`self.K2_GetPawn`))
  (bind _returnvalue (`|CreateWidget` "/Game/Player/Inventory/InventoryUI/HUD.HUD_C"))
  (bind _output_get (set `self.HUD_Widget` _returnvalue))
  (`UserWidget.AddToViewport` _output_get 0))

(fn `UserConstructionScript`)
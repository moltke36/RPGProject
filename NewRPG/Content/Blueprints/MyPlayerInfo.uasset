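; MyPlayerInfo tracks the player's enemy kill count and triggers a door opening once enough kills are reached.
; AddKillNumber increments EnemyKills and prints the new total as debug text.
; When the count is 15 or more and player 0's ThirdPersonCharacter has not died, it calls OpenDoor, which repeats on each further qualifying kill.
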(event `AddKillNumber`
  (bind _result (`/Engine/EditorBlueprintResources/StandardMacros.IncrementInt` (`self.EnemyKills`))
    (:`  `
      (`KismetSystemLibrary.PrintString` "GetKills")
      (`KismetSystemLibrary.PrintString` (`KismetStringLibrary.Conv_IntToString` _result))
      (if (and (>= (`self.EnemyKills`) 15) (not (`/Game/ThirdPersonBP/Blueprints/ThirdPersonCharacter.isDied?` (cast `/Game/ThirdPersonBP/Blueprints/ThirdPersonCharacter` (`GameplayStatics.GetPlayerPawn` 0) :!pure true))))
        (`self.OpenDoor`)))))

(fn `UserConstructionScript`)
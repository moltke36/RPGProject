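; Behavior tree node, likely a service, that updates an enemy's chase distances and ends the chase when it runs too far.
; Each AI tick with a FoundEnemy on the blackboard, it writes the pawn's distance to that target and to ChaseStartPoint into ChaseDistance and DistanceFromStart.
; It calls ClearTarget on the Enemy pawn when either distance exceeds that pawn's own MaxChaseDistance or FollowingDIstance limit, respectively.
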(event `self.ReceiveTickAI`
  (params (OwnerController :type "AIController Object Reference") (ControlledPawn :type "Pawn Object Reference") (DeltaSeconds :type "Float (single-precision)"))
  (bind _returnvalue (`Actor.K2_GetActorLocation` ControlledPawn))
  (bind _asenemy (cast `/Game/ThirdPersonBP/Blueprints/Enemy` ControlledPawn :!pure true))
  (bind _blackboard_comp (`self.Blackboard comp`))
  (bind (_asactor _bsuccess) (cast `Actor` (`BlackboardComponent.GetValueAsObject` (`self.Blackboard comp`) (`KismetStringLibrary.Conv_StringToName` "FoundEnemy")) :!pure true))
  (bind _returnvalue_2 (`KismetMathLibrary.Abs` (`KismetMathLibrary.VSize` (- (`BlackboardComponent.GetValueAsVector` _blackboard_comp (`KismetStringLibrary.Conv_StringToName` "ChaseStartPoint")) _returnvalue))))
  (bind _returnvalue_3 (`KismetMathLibrary.Abs` (`KismetMathLibrary.VSize` (- _returnvalue (`Actor.K2_GetActorLocation` _asactor)))))
  (set `self.Blackboard comp` (`AIBlueprintHelperLibrary.GetBlackboard` OwnerController))
  (if _bsuccess
    (`BlackboardComponent.SetValueAsFloat` _blackboard_comp (`KismetStringLibrary.Conv_StringToName` "ChaseDistance") _returnvalue_3)
    (`BlackboardComponent.SetValueAsFloat` _blackboard_comp (`KismetStringLibrary.Conv_StringToName` "DistanceFromStart") _returnvalue_2)
    (if (or (> _returnvalue_2 (`/Game/ThirdPersonBP/Blueprints/Enemy.MaxChaseDistance` _asenemy)) (> _returnvalue_3 (`/Game/ThirdPersonBP/Blueprints/Enemy.FollowingDIstance` _asenemy)))
      (`/Game/ThirdPersonBP/Blueprints/Enemy.ClearTarget` _asenemy))))
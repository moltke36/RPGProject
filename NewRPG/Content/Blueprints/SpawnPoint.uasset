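; Spawn point actor that keeps a population of enemies at its location, up to MaxRespawn.
; On BeginPlay it takes ownership of enemies already in SpawnedArray and starts spawning while below the limit.
; A timer calls SpawnEnemy after SpawnInterval, which spawns an owned enemy and re-arms the timer until full.
; RemoveEnemy drops an enemy from the array, restarts spawning and prunes invalid entries.
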(event `self.ReceiveBeginPlay`
  (bind _spawnedarray (`self.SpawnedArray`))
  ;[1 1 1] Set Array Character owner to self
  (if (!= (`KismetArrayLibrary.Array_Length` _spawnedarray) 0)
    (for _array_element _spawnedarray
      (`self.SetOwner` _array_element self))
    (if (< (`KismetArrayLibrary.Array_Length` (`self.SpawnedArray`)) (`self.MaxRespawn`))
      (set `self.KeepSpawn?` true)
      (`self.SpawnCharacter`))
    (else
      (set `self.KeepSpawn?` true)
      (`self.SpawnCharacter`))))

(event `SpawnCharacter`
  ;[1 1 1] SpawnEnemy
  (if (< (`KismetArrayLibrary.Array_Length` (`self.SpawnedArray`)) (`self.MaxRespawn`))
    (`KismetSystemLibrary.K2_SetTimer` null "SpawnEnemy" (`self.SpawnInterval`))
    (else
      (set `self.KeepSpawn?` false))))

(event `RemoveEnemy`
  (params (EnemyToRemove :type "Character Object Reference"))
  ;[1 1 1] ClearArray
  (`KismetArrayLibrary.Array_RemoveItem` (`self.SpawnedArray`) EnemyToRemove)
  (set `self.KeepSpawn?` true)
  (`self.SpawnCharacter`)
  (`self.CheckEmpty`))

(fn `CheckEmpty`
  (for _array_element (`self.SpawnedArray`)
    (if (not (`KismetSystemLibrary.IsValid` _array_element))
      (`KismetArrayLibrary.Array_RemoveItem` (`self.SpawnedArray`) _array_element))))

(fn `SpawnEnemy`
  (bind _returnvalue (`|SpawnActorFromClass` (`self.EnemyToSpawn`) (`self.GetTransform`) "AdjustIfPossibleButDontSpawnIfColliding" "OverrideRootScale" self null))
  (`KismetArrayLibrary.Array_Add` (`self.SpawnedArray`) _returnvalue)
  (`self.SpawnCharacter`))

(fn `UserConstructionScript`)